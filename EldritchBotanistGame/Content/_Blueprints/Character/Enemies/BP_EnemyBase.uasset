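; BP_EnemyBase is an enemy base Blueprint with health, damage handling and death.
; BeginPlay caches the WBP_Healthbar from its widget component, and AnyDamage passes truncated damage to TakeDamage.
; TakeDamage lowers Health, then, only if the healthbar is valid, updates its percent and calls Death at zero or below, destroying the actor.
; Tick, attack-range and capsule overlap events are empty.
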(event `self.ReceiveBeginPlay`
  (bind _aswbp_healthbar (cast `/Game/_Blueprints/UI/WBP_Healthbar` (`WidgetComponent.GetUserWidgetObject` (`self.WC_HealthBar`))))
  (set `self.WBP Healthbar` _aswbp_healthbar))

(event `self.ReceiveTick`
  (params (DeltaSeconds :type "Float (single-precision)")))

(event `self.AttackRange.OnComponentBeginOverlap`
  (params (OverlappedComponent :type "PrimitiveComponent Object Reference") (OtherActor :type "Actor Object Reference") (OtherComp :type "PrimitiveComponent Object Reference") (OtherBodyIndex :type Integer) (bFromSweep :type Boolean) (SweepResult :type "HitResult Structure (by ref)")))

(event `self.AttackRange.OnComponentEndOverlap`
  (params (OverlappedComponent :type "PrimitiveComponent Object Reference") (OtherActor :type "Actor Object Reference") (OtherComp :type "PrimitiveComponent Object Reference") (OtherBodyIndex :type Integer)))

(event `self.CapsuleComponent.OnComponentBeginOverlap`
  (params (OverlappedComponent :type "PrimitiveComponent Object Reference") (OtherActor :type "Actor Object Reference") (OtherComp :type "PrimitiveComponent Object Reference") (OtherBodyIndex :type Integer) (bFromSweep :type Boolean) (SweepResult :type "HitResult Structure (by ref)")))

(event `self.ReceiveAnyDamage`
  (params (Damage :type "Float (single-precision)") (DamageType :type "DamageType Object Reference") (InstigatedBy :type "Controller Object Reference") (DamageCauser :type "Actor Object Reference"))
  (`self.TakeDamage` (`KismetMathLibrary.FTrunc` Damage)))

(fn `Death`
  (`self.K2_DestroyActor`))

(fn `TakeDamage`
  (params (Amount :type Integer))
  (bind _wbp_healthbar (`self.WBP Healthbar`))
  (bind _output_get (set `self.Health` (- (`self.Health`) Amount)))
  (`/Engine/EditorBlueprintResources/StandardMacros.IsValid` _wbp_healthbar
    (:`Is Valid`
      (`/Game/_Blueprints/UI/WBP_Healthbar.SetPercent` _wbp_healthbar (`KismetMathLibrary.Conv_IntToDouble` (`self.MaxHealth`)) (`KismetMathLibrary.Conv_IntToDouble` _output_get))
      (if (<= _output_get 0)
        (`self.Death`)))))

(fn `UserConstructionScript`)