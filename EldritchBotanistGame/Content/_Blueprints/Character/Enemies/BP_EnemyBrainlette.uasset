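; BP_EnemyBrainlette is the Brainlette enemy character, a thin child Blueprint that leaves most of its behavior to its parent.
; On BeginPlay it assigns PF_Slash as its attack animation, then runs the parent's BeginPlay.
; ToggleAnimation disables or enables animation on both the mesh and its outline mesh according to IsStopped, keeping the two in step.
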(event `self.ReceiveBeginPlay`
  (set `self.AttackAnim` "/Game/_Sprites/Flipbooks/PF_Slash.PF_Slash")
  (`parent.ReceiveBeginPlay`))

(fn `ToggleAnimation`
  (if (`self.IsStopped?`)
    (`SkeletalMeshComponent.SetEnableAnimation` (`self.Mesh`) false)
    (`SkeletalMeshComponent.SetEnableAnimation` (`self.CharacterMesh_outline`) false)
    (else
      (`SkeletalMeshComponent.SetEnableAnimation` (`self.Mesh`) true)
      (`SkeletalMeshComponent.SetEnableAnimation` (`self.CharacterMesh_outline`) true))))

(fn `UserConstructionScript`
  (`parent.UserConstructionScript`))