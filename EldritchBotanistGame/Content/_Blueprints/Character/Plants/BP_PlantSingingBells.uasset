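; BP_PlantSingingBells is a plant character Blueprint that configures a healing effect based on the plant's level.
; On BeginPlay it runs the parent logic, then sets HealAmt on its BPCEffectInRange component to a base value, raised at levels 2 and 3.
; The component and parent class supply all other behavior, as overlap and tick events are disabled stubs.
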(event `self.ReceiveBeginPlay`
  (bind _bpc_effectinrange (`self.BPC_EffectInRange`))
  (`parent.ReceiveBeginPlay`)
  (set `/Game/_Blueprints/Character/Plants/BPC_EffectInRange.HealAmt` 3 _bpc_effectinrange)
  (if (== (`self.Level`) 2)
    (set `/Game/_Blueprints/Character/Plants/BPC_EffectInRange.HealAmt` 4 _bpc_effectinrange)
    (elif (== (`self.Level`) 3)
      (set `/Game/_Blueprints/Character/Plants/BPC_EffectInRange.HealAmt` 6 _bpc_effectinrange))))

(fn `UserConstructionScript`
  (`parent.UserConstructionScript`))