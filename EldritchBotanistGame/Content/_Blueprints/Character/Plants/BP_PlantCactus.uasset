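; BP_PlantCactus is a plant that does not attack on its own and instead hurts enemies when it is hit.
; Taking damage applies it to the plant, spawns a damage indicator and sets a short timer for Retaliation.
; Retaliation damages every BP_EnemyBase overlapping AttackRange.
; At level 3 and above it gains a charm charge at BeginPlay and also charms enemies through BPCEffectInRange when retaliating.
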(event `self.ReceiveBeginPlay`
  (if (>= (`self.Level`) 3)
    (set `/Game/_Blueprints/Character/Plants/BPC_EffectInRange.CharmCharges` 1 (`self.BPC_EffectInRange`)))
  (`parent.ReceiveBeginPlay`))

(event `self.BeginAttacking`
  ;[0 0 0 0.5] Instead of attacking...
)

(event `self.ReceiveAnyDamage`
  (params (Damage :type "Float (single-precision)") (DamageType :type "DamageType Object Reference") (InstigatedBy :type "Controller Object Reference") (DamageCauser :type "Actor Object Reference"))
  (bind _returnvalue_location (`KismetMathLibrary.BreakTransform` (`self.GetTransform`)))
  ;[0.3531 0 0 0.5] When attacked, hit all enemies in range
  (`self.TakeDamage` (`KismetMathLibrary.FTrunc` Damage))
  (`|SpawnActorFromClass` "/Game/_Blueprints/Character/HealthAndDamage/BP_DmgIndicator.BP_DmgIndicator_C" (`KismetMathLibrary.MakeTransform` (+ _returnvalue_location (65.0 -250.0 0.0))) "Undefined" "MultiplyWithRoot" null Damage false false null)
  (`KismetSystemLibrary.K2_SetTimer` null "Retaliation" 0.3))

(fn `Retaliation`
  (if (>= (`self.Level`) 3)
    (`/Game/_Blueprints/Character/Plants/BPC_EffectInRange.CharmEnemies` (`self.BPC_EffectInRange`) 1 false))
  (for _array_element (`PrimitiveComponent.GetOverlappingActors` (`self.AttackRange`) "/Game/_Blueprints/Character/Enemies/BP_EnemyBase.BP_EnemyBase_C")
    (`GameplayStatics.ApplyDamage` _array_element (`self.Damage`))))

(fn `UserConstructionScript`
  (`parent.UserConstructionScript`))