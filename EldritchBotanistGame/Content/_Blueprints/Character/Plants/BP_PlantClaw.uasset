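; BP_PlantClaw is the claw plant, a child plant Blueprint that configures a slow and attack-speed effect in range based on its level.
; On BeginPlay it sets the chomp attack animation, runs the parent logic and, after a short delay outside the main menu, plays its sound.
; Cascading level checks then overwrite the BPCEffectInRange values with stronger ones per tier, and the third tier also enables rage.
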(event `self.ReceiveBeginPlay`
  (bind _bpc_effectinrange (`self.BPC_EffectInRange`))
  (bind _bpc_effectinrange_2 (`self.BPC_EffectInRange`))
  (bind _bpc_effectinrange_3 (`self.BPC_EffectInRange`))
  (set `self.AttackAnim` "/Game/_Sprites/Flipbooks/PF_Chomp.PF_Chomp")
  (`parent.ReceiveBeginPlay`)
  (`KismetSystemLibrary.Delay` 0.1)
  (if (not (`self.IsMainMenu?`))
    (`GameplayStatics.PlaySound2D` "/Game/_Audio/Plant_SFX/claw_plant.claw_plant" 1.0 1.0 0.0 null null)
    (`|ExecutionSequence`
      (:`then_0`
        (if (>= (`self.Level`) 1)
          (set `/Game/_Blueprints/Character/Plants/BPC_EffectInRange.SlowAmt` 0.8 _bpc_effectinrange_2)
          (set `/Game/_Blueprints/Character/Plants/BPC_EffectInRange.AtkSpeedChange` 0.9 _bpc_effectinrange_2)))
      (:`then_1`
        (if (>= (`self.Level`) 2)
          (set `/Game/_Blueprints/Character/Plants/BPC_EffectInRange.SlowAmt` 0.7 _bpc_effectinrange_3)
          (set `/Game/_Blueprints/Character/Plants/BPC_EffectInRange.AtkSpeedChange` 0.8 _bpc_effectinrange_3)))
      (:`then_2`
        (if (>= (`self.Level`) 3)
          (set `/Game/_Blueprints/Character/Plants/BPC_EffectInRange.SlowAmt` 0.7 _bpc_effectinrange)
          (set `/Game/_Blueprints/Character/Plants/BPC_EffectInRange.AtkSpeedChange` 0.7 _bpc_effectinrange)
          (set `self.HasRage?` true))))))

(fn `UserConstructionScript`
  (`parent.UserConstructionScript`))