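; Actor component that periodically applies area buffs to plants and debuffs to enemies, including healing, attack, attack speed, slow, stop and charm.
; A looping cooldown timer fires CastEffect, which runs each effect whose tuning value is active.
; Effects use overlaps of the owning plant's PlantEffectRange; enemy owners are cached, but every effect reads the plant reference.
; Charm hits the nearest or all nearby enemies, assigning other enemies as attack targets.
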(event `self.ReceiveBeginPlay`
  (bind _returnvalue (`self.GetOwner`))
  (bind _asbp_plant_base (cast `/Game/_Blueprints/Character/Plants/BP_PlantBase` _returnvalue)
    (:`then`
      (set `self.PLANT_SELF_REF` _asbp_plant_base))
    (:`CastFailed`
      (bind _asbp_enemy_base (cast `/Game/_Blueprints/Character/Enemies/BP_EnemyBase` _returnvalue))
      (set `self.ENEMY_SELF_REF` _asbp_enemy_base)))
  (`KismetSystemLibrary.K2_SetTimerDelegate` (delegate `CastEffect`) (`self.Cooldown`) true))

(event `CastEffect`
  (bind _atkspeedchange (`self.AtkSpeedChange`))
  (bind _atkupamt (`self.AtkUpAmt`))
  (bind _healamt (`self.HealAmt`))
  (bind _atkdownamt (`self.AtkDownAmt`))
  (bind _slowamt (`self.SlowAmt`))
  (bind _stopcharges (`self.StopCharges`))
  (bind _charmcharges (`self.CharmCharges`))
  (`|ExecutionSequence`
    (:`then_0`
      ;[0 0 0 0.5] Allied Effects
      ;;[0.5406 0.01399 0.1151 0.5] Heal Nearby (PLANTS)
      (if (> _healamt 0)
        (`self.HealNearbyPlants` (`KismetMathLibrary.Conv_IntToDouble` _healamt))))
    (:`then_1`
      ;;[0.5281 0 0 0.5] Attack Up (PLANTS)
      (if (> _atkupamt 0)
        (`self.AttackUpNearbyPlants` _atkupamt)))
    (:`then_2`
      ;;[0.4323 0.01846 0.3756 0.5] Attack Speed Up (PLANTS)
      (if (< _atkspeedchange 1.0)
        ;[0 0 0 0.5] Enemy Effects
        ;;[0.4323 0.01846 0.3756 0.5] Attack Speed Down (ENEMIES)
        (`self.AtkSpdDownNearbyEnemies` _atkspeedchange)
        (elif (> _atkspeedchange 1.0)
          (`self.AtkSpdUpNearbyPlants` _atkspeedchange))))
    (:`then_3`
      (`|ExecutionSequence`
        (:`then_0`
          ;;[0.4323 0.01846 0.3756 0.5] Atk Down (Enemies)
          (if (> _atkdownamt 0)
            (`self.AtkDownNearbyEnemies` _atkdownamt)))
        (:`then_1`
          ;;[0.1682 0.4323 0.08634 0.5] Slow (Enemies)
          (if (< _slowamt 1.0)
            (`self.SlowNearbyEnemies` _slowamt)))
        (:`then_2`
          ;;[0.15 0.5409 0.15 0.5] Stop (Enemies)
          (if (> _stopcharges 0)
            (`self.StopNearbyEnemies` _stopcharges)))
        (:`then_3`
          ;;[0.3323 0.01623 0.201 0.5] Charm (ENEMIES)
          (if (> _charmcharges 0)
            (`self.CharmEnemies` _charmcharges)))))))

(fn `AtkDownNearbyEnemies`
  (params (AtkDownAmt :type Integer))
  (for _array_element (`PrimitiveComponent.GetOverlappingActors` (`/Game/_Blueprints/Character/Plants/BP_PlantBase.PlantEffectRange` (`self.PLANT_SELF_REF`)) "/Game/_Blueprints/Character/Enemies/BP_EnemyBase.BP_EnemyBase_C")
    (bind _asbp_enemy_base (cast `/Game/_Blueprints/Character/Enemies/BP_EnemyBase` _array_element))
    (`/Game/_Blueprints/Character/Enemies/BP_EnemyBase.AtkDown` _asbp_enemy_base AtkDownAmt)))

(fn `AtkSpdDownNearbyEnemies`
  (params (AtkSpeedDownAmt :type "Float (double-precision)"))
  (for _array_element (`PrimitiveComponent.GetOverlappingActors` (`/Game/_Blueprints/Character/Plants/BP_PlantBase.PlantEffectRange` (`self.PLANT_SELF_REF`)) "/Game/_Blueprints/Character/Enemies/BP_EnemyBase.BP_EnemyBase_C")
    (bind _asbp_enemy_base (cast `/Game/_Blueprints/Character/Enemies/BP_EnemyBase` _array_element))
    (`/Game/_Blueprints/Character/Enemies/BP_EnemyBase.AtkSpeedDown` _asbp_enemy_base AtkSpeedDownAmt)))

(fn `AtkSpdUpNearbyPlants`
  (params (AtkSpeedUpAmt :type "Float (double-precision)"))
  (for _array_element (`PrimitiveComponent.GetOverlappingActors` (`/Game/_Blueprints/Character/Plants/BP_PlantBase.PlantEffectRange` (`self.PLANT_SELF_REF`)) "/Game/_Blueprints/Character/Plants/BP_PlantBase.BP_PlantBase_C")
    (bind _asbp_plant_base (cast `/Game/_Blueprints/Character/Plants/BP_PlantBase` _array_element))
    (`/Game/_Blueprints/Character/Plants/BP_PlantBase.AttackSpeedUp` _asbp_plant_base AtkSpeedUpAmt)))

(fn `AttackUpNearbyPlants`
  (params (AtkUpAmt :type Integer))
  (for _array_element (`PrimitiveComponent.GetOverlappingActors` (`/Game/_Blueprints/Character/Plants/BP_PlantBase.PlantEffectRange` (`self.PLANT_SELF_REF`)) "/Game/_Blueprints/Character/Plants/BP_PlantBase.BP_PlantBase_C")
    (bind _asbp_plant_base (cast `/Game/_Blueprints/Character/Plants/BP_PlantBase` _array_element))
    (`/Game/_Blueprints/Character/Plants/BP_PlantBase.AttackUp` _asbp_plant_base AtkUpAmt)))

(fn `CharmEnemies`
  (params (AddCharmCharge :type Integer))
  (locals (AllButNearest :type "Array of Actor Object Reference") (AllNearby :type "Array of Actor Object Reference") (Nearest :type "Actor Object Reference") (SecondNearest :type "Actor Object Reference"))
  (bind _plant_self_ref (`self.PLANT_SELF_REF`))
  (bind _returnvalue (`Actor.K2_GetActorLocation` _plant_self_ref))
  (bind _overlappingactors (`PrimitiveComponent.GetOverlappingActors` (`/Game/_Blueprints/Character/Plants/BP_PlantBase.PlantEffectRange` _plant_self_ref) "/Game/_Blueprints/Character/Enemies/BP_EnemyBase.BP_EnemyBase_C"))
  (set `local.AllNearby` _overlappingactors)
  (bind _output_get (set `local.Nearest` (`.ReturnValue` (`GameplayStatics.FindNearestActor` _returnvalue _overlappingactors))))
  (bind _outactors (`GameplayStatics.GetAllActorsOfClass` "/Game/_Blueprints/Character/Enemies/BP_EnemyBase.BP_EnemyBase_C"))
  (bind _output_get_2 (set `local.AllButNearest` _outactors))
  (`KismetArrayLibrary.Array_RemoveItem` _output_get_2 _output_get)
  (set `local.SecondNearest` (`.ReturnValue` (`GameplayStatics.FindNearestActor` _returnvalue (`local.AllButNearest`))))
  (if (`self.CharmAllNearby?`)
    (for _array_element (`local.AllNearby`)
      (bind _asbp_enemy_base (cast `/Game/_Blueprints/Character/Enemies/BP_EnemyBase` _array_element))
      (`/Game/_Blueprints/Character/Enemies/BP_EnemyBase.Charm` _asbp_enemy_base AddCharmCharge (`local.Nearest`) (`local.SecondNearest`)))
    (else
      (bind _asbp_enemy_base_2 (cast `/Game/_Blueprints/Character/Enemies/BP_EnemyBase` (`local.Nearest`)))
      (`/Game/_Blueprints/Character/Enemies/BP_EnemyBase.Charm` _asbp_enemy_base_2 AddCharmCharge (`local.SecondNearest`) null)))
  (return))

(fn `HealNearbyPlants`
  (params (HealAmt :type "Float (double-precision)"))
  (for _array_element (`PrimitiveComponent.GetOverlappingActors` (`/Game/_Blueprints/Character/Plants/BP_PlantBase.PlantEffectRange` (`self.PLANT_SELF_REF`)) "/Game/_Blueprints/Character/Plants/BP_PlantBase.BP_PlantBase_C")
    (bind _asbp_plant_base (cast `/Game/_Blueprints/Character/Plants/BP_PlantBase` _array_element))
    (`/Game/_Blueprints/Character/Plants/BP_PlantBase.Heal` _asbp_plant_base HealAmt)))

(fn `SlowNearbyEnemies`
  (params (SpeedDownAmt :type "Float (double-precision)"))
  (for _array_element (`PrimitiveComponent.GetOverlappingActors` (`/Game/_Blueprints/Character/Plants/BP_PlantBase.PlantEffectRange` (`self.PLANT_SELF_REF`)) "/Game/_Blueprints/Character/Enemies/BP_EnemyBase.BP_EnemyBase_C")
    (bind _asbp_enemy_base (cast `/Game/_Blueprints/Character/Enemies/BP_EnemyBase` _array_element))
    (`/Game/_Blueprints/Character/Enemies/BP_EnemyBase.Slow` _asbp_enemy_base SpeedDownAmt)))

(fn `StopNearbyEnemies`
  (params (AddStopCharge :type Integer))
  (for _array_element (`PrimitiveComponent.GetOverlappingActors` (`/Game/_Blueprints/Character/Plants/BP_PlantBase.PlantEffectRange` (`self.PLANT_SELF_REF`)) "/Game/_Blueprints/Character/Enemies/BP_EnemyBase.BP_EnemyBase_C")
    (bind _asbp_enemy_base (cast `/Game/_Blueprints/Character/Enemies/BP_EnemyBase` _array_element))
    (`/Game/_Blueprints/Character/Enemies/BP_EnemyBase.Stop` _asbp_enemy_base AddStopCharge)))