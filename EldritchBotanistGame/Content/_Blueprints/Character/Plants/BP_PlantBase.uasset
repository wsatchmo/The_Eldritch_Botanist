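; Base plant actor that acts as an auto-targeting turret against BP_EnemyBase actors.
; Each tick it picks the nearest enemy overlapping AttackRange, draws a debug sphere on it and gradually rotates toward a point slightly below its origin.
; A looping FireRate timer spawns BP_Projectile aimed directly at that point, independent of the plant's current rotation.
; Damage handling only prints a message.
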(event `self.ReceiveBeginPlay`
  ;[0.3165 0 0.005331 0.5] Spawn Projectile to fire at target
  (`KismetSystemLibrary.K2_SetTimerDelegate` (delegate `Fire`) (`self.FireRate`) true))

(event `Fire`
  (bind _returnvalue (`self.K2_GetActorLocation`))
  ;[0.3165 0 0.005331 0.5] Spawn Projectile to fire at target
  (bind _settarget (`self.SetTarget`)
    (:`then`
      (`|SpawnActorFromClass` "/Game/_Blueprints/Character/BP_Projectile.BP_Projectile_C" (`KismetMathLibrary.MakeTransform` _returnvalue (`KismetMathLibrary.FindLookAtRotation` _returnvalue (- (`self.K2_GetActorLocation` _settarget) (0.0 0.0 35.0)))) "Undefined" "MultiplyWithRoot" null 20 null))
    (:`else`)))

(event `self.ReceiveTick`
  (params (DeltaSeconds :type "Float (single-precision)"))
  ;[0.299 0.03021 0.03021 0.5] Set Target and Rotate Toward
  (bind _output_get (set `self.SetTarget` (`self.GetClosestTarget`)))
  (`/Engine/EditorBlueprintResources/StandardMacros.IsValid` _output_get
    (:`Is Valid`
      (`KismetSystemLibrary.DrawDebugSphere` (`self.K2_GetActorLocation` _output_get) 50.0)
      (bind _returnvalue (`KismetMathLibrary.RInterpTo` (`self.K2_GetActorRotation`) (`KismetMathLibrary.FindLookAtRotation` (`self.K2_GetActorLocation`) (- (`self.K2_GetActorLocation` (stale `Fire` _settarget)) (0.0 0.0 35.0))) 1.0 0.05))
      (`self.K2_SetActorRotation` _returnvalue))))

(event `self.ReceiveAnyDamage`
  (params (Damage :type "Float (single-precision)") (DamageType :type "DamageType Object Reference") (InstigatedBy :type "Controller Object Reference") (DamageCauser :type "Actor Object Reference"))
  (`KismetSystemLibrary.PrintString` "Taking damage"))

(fn `GetClosestTarget`
  (returns (ClosestEnemy :type "Actor Object Reference"))
  (locals (LocDistance :type "Array of Float (double-precision)"))
  (bind _overlappingactors (`PrimitiveComponent.GetOverlappingActors` (`self.AttackRange`) "/Game/_Blueprints/Character/Enemies/BP_EnemyBase.BP_EnemyBase_C"))
  (switch `int` (`KismetArrayLibrary.Array_Length` _overlappingactors)
    (:`Default`
      (for _array_element _overlappingactors
        (`KismetArrayLibrary.Array_Add` (`local.LocDistance`) (`KismetMathLibrary.Vector_Distance` (`self.K2_GetActorLocation` _array_element) (`self.K2_GetActorLocation`))))
      (return (`|GetArrayItem` _overlappingactors (`KismetMathLibrary.MinOfFloatArray` (`local.LocDistance`)))))
    (:`0`
      (return null))
    (:`1`
      (return (`|GetArrayItem` _overlappingactors)))))

(fn `UserConstructionScript`)