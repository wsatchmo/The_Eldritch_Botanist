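; A poison spit projectile that poisons and damages the enemies it overlaps.
; On spawn it plays a spit sound and a brief poison flipbook on PurpleBubble, then destroys itself after a timeout.
; Sphere overlap with a BP_EnemyBase applies poison and Damage, replays the flipbook, hides the mesh and destroys the actor after a short delay.
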(event `self.ReceiveBeginPlay`
  (`GameplayStatics.PlaySound2D` "/Game/_Audio/AttackSFX/AttackSpit.AttackSpit" 2.4 1.0 0.0 null null)
  (`PaperFlipbookComponent.SetFlipbook` (`self.PurpleBubble`) "/Game/_Sprites/Flipbooks/PF_SpitPoison.PF_SpitPoison")
  (`KismetSystemLibrary.Delay` 0.5)
  (`PaperFlipbookComponent.SetFlipbook` (`self.PurpleBubble`) null)
  (`KismetSystemLibrary.Delay` 10.0)
  (`self.K2_DestroyActor`))

(event `self.Sphere.OnComponentBeginOverlap`
  (params (OverlappedComponent :type "PrimitiveComponent Object Reference") (OtherActor :type "Actor Object Reference") (OtherComp :type "PrimitiveComponent Object Reference") (OtherBodyIndex :type Integer) (bFromSweep :type Boolean) (SweepResult :type "HitResult Structure (by ref)"))
  (bind _purplebubble (`self.PurpleBubble`))
  (bind _asbp_enemy_base (cast `/Game/_Blueprints/Character/Enemies/BP_EnemyBase` OtherActor))
  (`/Game/_Blueprints/Character/Enemies/BP_EnemyBase.ApplyPoison` _asbp_enemy_base 12.5)
  (`GameplayStatics.ApplyDamage` _asbp_enemy_base (`KismetMathLibrary.Conv_IntToDouble` (`self.Damage`)))
  (`PaperFlipbookComponent.SetFlipbook` _purplebubble "/Game/_Sprites/Flipbooks/PF_SpitPoison.PF_SpitPoison")
  (`PaperFlipbookComponent.Play` _purplebubble)
  (`SceneComponent.SetVisibility` (`self.StaticMesh`) false false)
  (`KismetSystemLibrary.Delay` 0.5)
  (`self.K2_DestroyActor`))

(fn `UserConstructionScript`)