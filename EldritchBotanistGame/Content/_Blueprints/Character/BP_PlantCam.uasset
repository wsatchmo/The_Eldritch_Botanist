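; Plant camera actor that spawns a plant for inspection and owns the day cycle UI, which it creates on BeginPlay.
; StoreCurrentPlant caches the plant's data, and SpawnPlantFromData, gated by CanSummon, replaces the previous plant at the camera's transform.
; Tick pushes the stored name and info into the UI's inspection table.
; The construction script adds the actor itself to the scene capture's show-only list.
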(event `self.ReceiveBeginPlay`
  ;[0.08273 0.08782 0.4487 0.5] Create Day Widgets (OWNED BY PLANTCAM)
  (bind _returnvalue (`|CreateWidget` "/Game/_Blueprints/UI/DayUI/WBP_DayCycleUI.WBP_DayCycleUI_C"))
  (set `self.DayCycleUIRef` _returnvalue)
  (`UserWidget.AddToViewport` _returnvalue 0))

(event `SpawnPlantFromData`
  (bind (_returnvalue_location _returnvalue_rotation) (`KismetMathLibrary.BreakTransform` (`self.GetTransform`)))
  ;[0.15 0.4991 0.15 0.5] Spawn Actor from Button, set 'Can Summon' to false
  (if (`self.CanSummon`)
    ;; Get what is already there and delete (WHY NOT WORKING??) -- else, get a reference to it on build
    ;; Because it isnt by ID???
    (`self.K2_DestroyActor` (`self.SpawnedPlant`))
    (bind _returnvalue (`|SpawnActorFromClass` "/Game/_Blueprints/Character/Plants/BP_PlantBase.BP_PlantBase_C" (`KismetMathLibrary.MakeTransform` _returnvalue_location _returnvalue_rotation) "Undefined" "MultiplyWithRoot" null (`self.PlantName`) 0 null))
    (set `self.SpawnedPlant` _returnvalue)))

(event `self.ReceiveTick`
  (params (DeltaSeconds :type "Float (single-precision)"))
  (bind _wbp_inspectiontable (`/Game/_Blueprints/UI/DayUI/WBP_DayCycleUI.WBP_InspectionTable` (`self.DayCycleUIRef`)))
  ;[0.05807 0.0422 0.4323 0.5] Set info on UI
  (`RichTextBlock.SetText` (`/Game/_Blueprints/UI/DayUI/WBP_InspectionTable.TYPENAME_TEXT` _wbp_inspectiontable) (`KismetTextLibrary.Conv_StringToText` (`self.PlantName`)))
  (`RichTextBlock.SetText` (`/Game/_Blueprints/UI/DayUI/WBP_InspectionTable.PLANTINFO_TEXT` _wbp_inspectiontable) (`KismetTextLibrary.Conv_StringToText` (`self.PlantInfo`))))

(fn `SpawnPlant`
  (bind (_returnvalue_location _returnvalue_rotation) (`KismetMathLibrary.BreakTransform` (`self.GetTransform`)))
  (`KismetSystemLibrary.PrintString` "Hello")
  (`|SpawnActorFromClass` "/Game/_Blueprints/Character/Plants/BP_PlantBase.BP_PlantBase_C" (`KismetMathLibrary.MakeTransform` _returnvalue_location _returnvalue_rotation) "AdjustIfPossibleButAlwaysSpawn" "MultiplyWithRoot" null "" 0 null))

(fn `StoreCurrentPlant`
  (params (SpawnedPlant :type "/Game/_Blueprints/Character/Plants/BP_PlantBase Object Reference") (PlantID :type Name) (PlantName :type String) (PlantInfo :type String) (PlantIngredients :type "Map of String to Integer") (ButtonName :type "/Game/_Blueprints/UI/Greenhouse/UMG_GreenhouseItemDay Object Reference"))
  (`|ExecutionSequence`
    (:`then_0`
      (set `self.SpawnedPlant` SpawnedPlant))
    (:`then_1`
      (set `self.PlantID` PlantID))
    (:`then_2`
      (set `self.PlantName` PlantName))
    (:`then_3`
      (set `self.PlantInfo` PlantInfo))
    (:`then_4`
      (set `self.PlantIngredients` PlantIngredients))
    (:`then_5`
      (set `self.ButtonName` ButtonName))))

(fn `UserConstructionScript`
  (cast `/Game/_Blueprints/Inventory/BP_PlantDataStore` (`self.PlantDataStoreRef`))
  (`SceneCaptureComponent.ShowOnlyActorComponents` (`self.SceneCaptureComponent2D`) self false))