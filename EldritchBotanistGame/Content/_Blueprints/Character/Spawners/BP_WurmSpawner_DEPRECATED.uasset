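; Deprecated spawner actor that spawns a limited number of BP_EnemyWurm enemies at its own location and rotation.
; After an initial delay on BeginPlay, a self-calling SpawnEnemy event spawns one wurm, increments a counter and waits a set interval before repeating until the target amount is reached.
; Spawns adjust for collisions but always happen.
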(event `self.ReceiveBeginPlay`
  ;[0.4574 0 0 0.5] Spawning Enemies
  (`KismetSystemLibrary.Delay` (`self.SpawnDelay`))
  (`self.SpawnEnemy`))

(event `SpawnEnemy`
  (bind (_returnvalue_location _returnvalue_rotation) (`KismetMathLibrary.BreakTransform` (`self.GetTransform`)))
  ;[0.4574 0 0 0.5] Spawning Enemies
  (if (< (`self.AmtSpawned`) (`self.AmtToSpawn`))
    (`|SpawnActorFromClass` :`Class` "/Game/_Blueprints/Character/Enemies/BP_EnemyWurm.BP_EnemyWurm_C" :`SpawnTransform` (`KismetMathLibrary.MakeTransform` _returnvalue_location _returnvalue_rotation) :`CollisionHandlingOverride` "AdjustIfPossibleButAlwaysSpawn" :`TransformScaleMethod` "MultiplyWithRoot" :`AICEnemyRef` null :`Instigator` null)
    (set `self.AmtSpawned` (+ (`self.AmtSpawned`) 1))
    (`KismetSystemLibrary.Delay` (`self.DelayTime`))
    (`self.SpawnEnemy`)))

(fn `UserConstructionScript`)