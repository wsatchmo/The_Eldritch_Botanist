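; BP_EnemySpawner is a spawner actor that creates a limited number of random enemies at its own location.
; SpawnEnemy spawns a random class from TypesToSpawn, counts it, then calls SetSpawnerTimer.
; SetSpawnerTimer schedules SpawnEnemy again after a random delay until AmtToSpawn is reached; nothing here starts the first cycle.
; The sequential, non-random spawn branch is disconnected and never runs.
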(event `SpawnEnemy`
  (bind (_returnvalue_location _returnvalue_rotation) (`KismetMathLibrary.BreakTransform` (`self.GetTransform`)))
  (bind _typestospawn (`self.TypesToSpawn`))
  ;[0.4574 0 0 0.5] Spawning Enemies
  ;[0.449 0.08395 0.3771 0.5] For Random Spawning
  (`|SpawnActorFromClass` :`Class` (`|GetArrayItem` _typestospawn (`KismetMathLibrary.RandomIntegerInRange` 0 (- (`KismetArrayLibrary.Array_Length` _typestospawn) 1))) :`SpawnTransform` (`KismetMathLibrary.MakeTransform` _returnvalue_location _returnvalue_rotation) :`CollisionHandlingOverride` "AdjustIfPossibleButAlwaysSpawn" :`TransformScaleMethod` "MultiplyWithRoot" :`Instigator` null)
  (set `self.AmtSpawned` (+ (`self.AmtSpawned`) 1))
  (`self.SetSpawnerTimer`))

(fn `SetSpawnerTimer`
  (`KismetSystemLibrary.K2_ClearAndInvalidateTimerHandle` (`self.SpawnTimerHandle`))
  (if (not (>= (`self.AmtSpawned`) (`self.AmtToSpawn`)))
    (bind _returnvalue (`KismetSystemLibrary.K2_SetTimer` null "SpawnEnemy" (`KismetMathLibrary.RandomFloatInRange` (`self.MinTimeBetweenSummons`) (`self.MaxTimeBetweenSummons`))))
    (set `self.SpawnTimerHandle` _returnvalue)))

(fn `UserConstructionScript`)