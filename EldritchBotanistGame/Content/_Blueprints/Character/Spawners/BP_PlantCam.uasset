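; BP_PlantCam is a scene-capture actor that displays a selected plant for the day-cycle greenhouse UI, which it creates and owns.
; Button-driven spawning replaces the previous plant at the actor's location and, on one table, updates next/previous arrows.
; Stored plant stats and hints are pushed to the inspection table every Tick.
; It also maintains the crafting-table item array, with debug prints.
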(event `self.ReceiveBeginPlay`
  ;[0.08273 0.08782 0.4487 0.5] Create Day Widgets (OWNED BY PLANTCAM)
  (bind _returnvalue (`|CreateWidget` "/Game/_Blueprints/UI/DayUI/WBP_DayCycleUI.WBP_DayCycleUI_C" null null null null null null)) ; Own the Day Cycle UI
  (set `self.DayCycleUIRef` _returnvalue) ; Own the Cay Cycle UI
  (`UserWidget.AddToViewport` _returnvalue 0))

(event `self.ReceiveTick`
  (params (DeltaSeconds :type "Float (single-precision)"))
  ;[0.05807 0.0422 0.4323 0.5] Set info on UI -- EVENT TICK
  (`/Game/_Blueprints/UI/DayUI/Tables/WBP_InspectionTable.SetAllTexts` (`/Game/_Blueprints/UI/DayUI/WBP_DayCycleUI.WBP_InspectionTable` (`self.DayCycleUIRef`)) (`self.PlantName`) (`self.Plant Level`) (`self.PlantInfo`) (`self.Hint 1`) (`self.Hint 2`) (`self.Hint 3`) (`self.HP`) (`self.Attack`) (`self.Atk Speed`)) ; Set Inspection Table Values
)

(event `SetPlantValues`
  (params (PlantName :type String) (PlantLevel :type Integer) (PlantInfo :type String) (HP :type Integer) (Attack :type Integer) (AtkSpeed :type "Float (double-precision)") (ShowIngredients :type Boolean) (Hint1 :type String) (Hint2 :type String) (Hint3 :type String) (PlantType :type "/Game/_Blueprints/Data/E_PlantID Enum" :default "NewEnumerator11"))
  ;[0.01957 0.152 1 0.5] SET PLANT VALUES FOR UI
  (set `self.Plant ID` PlantType)
  (`|ExecutionSequence`
    (:`then_0`
      (set `self.PlantName` PlantName)
      (set `self.Plant Level` PlantLevel)
      (set `self.PlantInfo` PlantInfo))
    (:`then_1`
      (set `self.HP` HP)
      (set `self.Attack` Attack)
      (set `self.Atk Speed` AtkSpeed))
    (:`then_2`
      (set `self.Show Ingredients?` ShowIngredients)
      (set `self.Hint 1` Hint1)
      (set `self.Hint 2` Hint2)
      (set `self.Hint 3` Hint3))))

(event `AddCraftingTableItem`
  (params (`Item Added` :type "/Game/_Blueprints/Data/e_ResourceID Enum" :default "NewEnumerator0"))
  (bind _craftingtableitems (`self.CraftingTableItems`))
  ;[0.4365 0.2149 0.02166 0.5] Events handling the Crafting Table Items array
  (`KismetArrayLibrary.Array_Add` _craftingtableitems `Item Added`)
  (for _array_element _craftingtableitems
    (`KismetSystemLibrary.PrintString` (`KismetStringLibrary.Concat_StrStr` "Item in inventory: " (`|GetEnumeratorNameAsString` _array_element)))))

(event `SpawnPlantFromData`
  (params (Button :type "/Game/_Blueprints/UI/DayUI/Greenhouse/UMG_GreenhouseItemDay Object Reference"))
  (bind (_returnvalue_location _returnvalue_rotation) (`KismetMathLibrary.BreakTransform` (`self.GetTransform`)))
  (bind _daycycleuiref (`self.DayCycleUIRef`))
  (bind _spawnedplant (`self.SpawnedPlant`))
  (bind _wbp_nextlastbuttons_ (`/Game/_Blueprints/UI/DayUI/WBP_DayCycleUI.WBP_NextLastButtons_` _daycycleuiref))
  ;[0.15 0.4991 0.15 0.5] Spawn Actor in the PlantCam -- only needs actor class. Other information goes elsewhere
  (if (`self.CanSummon`)
    (if (`KismetSystemLibrary.IsValid` _spawnedplant)
      (`self.K2_DestroyActor` _spawnedplant))
    (bind _returnvalue (`|SpawnActorFromClass` (`/Game/_Blueprints/UI/DayUI/Greenhouse/UMG_GreenhouseItemDay.ClassRef` Button) (`KismetMathLibrary.MakeTransform` _returnvalue_location _returnvalue_rotation) "Undefined" "MultiplyWithRoot" null "" 0 110 30.0 30.0 1.0 1.0 0.9 110 false null))
    (`Widget.SetVisibility` (`/Game/_Blueprints/UI/DayUI/Tables/WBP_3DOverlay.DropS` (`/Game/_Blueprints/UI/DayUI/Tables/WBP_InspectionTable.WBP_3DOverlay` (`/Game/_Blueprints/UI/DayUI/WBP_DayCycleUI.WBP_InspectionTable` (`self.DayCycleUIRef`)))) "Visible")
    (set `self.SpawnedPlant` _returnvalue)
    (set `/Game/_Blueprints/UI/DayUI/Greenhouse/UMG_Greenhouse_Day.CurrButton` Button (`/Game/_Blueprints/UI/DayUI/WBP_DayCycleUI.UMG_Greenhouse_Landscape` _daycycleuiref))
    ;;[0.01358 0.06979 0.01887 0.5] Make Arrows (Only if on InspectionTable)
    (if (`|EnumEquality` (`/Game/_Blueprints/UI/DayUI/WBP_DayCycleUI.CurrTable` (`self.DayCycleUIRef`)) "NewEnumerator0")
      (`Widget.SetVisibility` _wbp_nextlastbuttons_ "Visible")
      (set `/Game/_Blueprints/UI/DayUI/Tables/WBP_NextLastButtons.HasItem?` true _wbp_nextlastbuttons_)
      (`self.SetNextLastButton`))))

(event `RemoveCraftingTableItem`
  (params (`Item Removed` :type "/Game/_Blueprints/Data/e_ResourceID Enum" :default "NewEnumerator0"))
  (bind _craftingtableitems (`self.CraftingTableItems`))
  ;[0.4365 0.2149 0.02166 0.5] Events handling the Crafting Table Items array
  (`KismetArrayLibrary.Array_Remove` _craftingtableitems (`KismetArrayLibrary.Array_Find` _craftingtableitems `Item Removed`))
  (`KismetSystemLibrary.PrintString` (`KismetStringLibrary.Concat_StrStr` "Item removed: " (`|GetEnumeratorNameAsString` `Item Removed`))))

(event `ClearCraftingTableArr`
  ;[0.4365 0.2149 0.02166 0.5] Events handling the Crafting Table Items array
  (`KismetArrayLibrary.Array_Clear` (`self.CraftingTableItems`)))

(fn `InitNextLastButton`
  (params (FirstInIndex :type "/Game/_Blueprints/UI/DayUI/Greenhouse/UMG_GreenhouseItemDay Object Reference"))
  (bind _wbp_nextlastbuttons_ (`/Game/_Blueprints/UI/DayUI/WBP_DayCycleUI.WBP_NextLastButtons_` (`self.DayCycleUIRef`)))
  (bind _output_get (set `/Game/_Blueprints/UI/DayUI/Tables/WBP_NextLastButtons.NextB_Item` FirstInIndex _wbp_nextlastbuttons_))
  (set `/Game/_Blueprints/UI/DayUI/Tables/WBP_NextLastButtons.LastB_Item` _output_get _wbp_nextlastbuttons_))

(fn `SetNextLastButton`
  (bind _daycycleuiref (`self.DayCycleUIRef`))
  (bind (_lastbutton _nextbutton _currentindex) (`/Game/_Blueprints/UI/DayUI/Greenhouse/UMG_Greenhouse_Day.GetCurrLastNextIndices` (`/Game/_Blueprints/UI/DayUI/WBP_DayCycleUI.UMG_Greenhouse_Landscape` _daycycleuiref)))
  (`/Game/_Blueprints/UI/DayUI/Tables/WBP_NextLastButtons.SetButtonValues` (`/Game/_Blueprints/UI/DayUI/WBP_DayCycleUI.WBP_NextLastButtons_` _daycycleuiref) _lastbutton _nextbutton _currentindex))

(fn `UserConstructionScript`
  (cast `/Game/_Blueprints/Inventory/BP_PlantDataStore` (`self.PlantDataStoreRef`))
  (`SceneCaptureComponent.ShowOnlyActorComponents` (`self.SceneCaptureComponent2D`) self false))