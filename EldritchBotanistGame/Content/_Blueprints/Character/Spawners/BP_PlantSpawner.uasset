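; BP_PlantSpawner is an actor that spawns a plant at its own transform when its spawn button widget is clicked.
; On BeginPlay it binds to the WBP_SpawnButton in its widget component and finds the BP_PlantDataStore actor.
; A click spawns the data store's ActorClass, then greys out and disables the button instance held there.
; A separate SpawnPlant function prints a debug string and spawns BP_PlantBase, without being called here.
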(event `self.ReceiveBeginPlay`
  ;[0.3861 0.04854 0.3393 0.5] Bind the button click to the Spawning Event
  (bind _aswbp_spawn_button (cast `/Game/_Blueprints/UI/WBP_SpawnButton` (`WidgetComponent.GetUserWidgetObject` (`self.WC_SpawnPlant`))))
  (add `/Game/_Blueprints/UI/WBP_SpawnButton.OnSpawnClicked` _aswbp_spawn_button (delegate `SpawnPlantFromData`)) ; In WBP_SpawnButton
  ;[0.4696 0.06864 0.3005 0.5] Set Plant Data Store to Variable
  (bind _returnvalue (`GameplayStatics.GetActorOfClass` "/Game/_Blueprints/Inventory/BP_PlantDataStore.BP_PlantDataStore_C"))
  (set `self.PlantDataStoreRef` _returnvalue))

(event `SpawnPlantFromData`
  (bind (_returnvalue_location _returnvalue_rotation) (`KismetMathLibrary.BreakTransform` (`self.GetTransform`)))
  (bind _plantdatastoreref (`self.PlantDataStoreRef`))
  (bind _buttoninstance (`/Game/_Blueprints/Inventory/BP_PlantDataStore.ButtonInstance` _plantdatastoreref))
  ;[0.15 0.4991 0.15 0.5] Spawn Actor from Button
  (`|SpawnActorFromClass` (`/Game/_Blueprints/Inventory/BP_PlantDataStore.ActorClass` _plantdatastoreref) (`KismetMathLibrary.MakeTransform` _returnvalue_location _returnvalue_rotation) "Undefined" "MultiplyWithRoot" null "" 0 null)
  (`UserWidget.SetColorAndOpacity` _buttoninstance (struct :`R` 0.311458 :`G` 0.311458 :`B` 0.311458 :`A` 0.488696))
  (set `/Game/_Blueprints/UI/Greenhouse/UMG_GreenhouseItemNight.IsClickable` false _buttoninstance))

(fn `SpawnPlant`
  (bind (_returnvalue_location _returnvalue_rotation) (`KismetMathLibrary.BreakTransform` (`self.GetTransform`)))
  (`KismetSystemLibrary.PrintString` "Hello")
  (`|SpawnActorFromClass` "/Game/_Blueprints/Character/Plants/BP_PlantBase.BP_PlantBase_C" (`KismetMathLibrary.MakeTransform` _returnvalue_location _returnvalue_rotation) "AdjustIfPossibleButAlwaysSpawn" "MultiplyWithRoot" null "" 0 null))

(fn `UserConstructionScript`
  (cast `/Game/_Blueprints/Inventory/BP_PlantDataStore` (`self.PlantDataStoreRef`)))