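; BP_Projectile is a spit projectile that damages BP_EnemyBase actors on overlap.
; On spawn it plays the spit sound and briefly shows a Paper2D spit flipbook, then destroys itself after a timed lifetime.
; A sphere overlap with an enemy applies Damage, replays the flipbook, hides the static mesh and destroys the actor after a short delay.
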(event `self.ReceiveBeginPlay`
  (`GameplayStatics.PlaySound2D` "/Game/_Audio/AttackSFX/AttackSpit.AttackSpit" 2.4 1.0 0.0 null null)
  (`PaperFlipbookComponent.SetFlipbook` (`self.PF_GreenBubble`) "/Game/_Sprites/Flipbooks/PF_Spit.PF_Spit")
  (`KismetSystemLibrary.Delay` 0.5)
  (`PaperFlipbookComponent.SetFlipbook` (`self.PF_GreenBubble`) null)
  (`KismetSystemLibrary.Delay` 10.0)
  (`self.K2_DestroyActor`))

(event `self.Sphere.OnComponentBeginOverlap`
  (params (OverlappedComponent :type "PrimitiveComponent Object Reference") (OtherActor :type "Actor Object Reference") (OtherComp :type "PrimitiveComponent Object Reference") (OtherBodyIndex :type Integer) (bFromSweep :type Boolean) (SweepResult :type "HitResult Structure (by ref)"))
  (bind _pf_greenbubble (`self.PF_GreenBubble`))
  (bind _asbp_enemy_base (cast `/Game/_Blueprints/Character/Enemies/BP_EnemyBase` OtherActor))
  (`/Engine/EditorBlueprintResources/StandardMacros.IsValid` _asbp_enemy_base
    (:`Is Valid`
      (`GameplayStatics.ApplyDamage` _asbp_enemy_base (`KismetMathLibrary.Conv_IntToDouble` (`self.Damage`)))
      (`PaperFlipbookComponent.SetFlipbook` _pf_greenbubble "/Game/_Sprites/Flipbooks/PF_Spit.PF_Spit")
      (`PaperFlipbookComponent.Play` _pf_greenbubble)
      (`SceneComponent.SetVisibility` (`self.StaticMesh`) false false)
      (`KismetSystemLibrary.Delay` 0.5)
      (`self.K2_DestroyActor`))))

(fn `UserConstructionScript`)