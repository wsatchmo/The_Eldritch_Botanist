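; BP_TDCamera is a movable camera pawn, apparently top-down, driven by Enhanced Input and touch swipes.
; BeginPlay adds the default and night-control mapping contexts, and IA_Move feeds movement input along the actor's forward and right vectors.
; A swipe past TouchMoveThreshold prints its direction, jumps the actor in world X or Y by the scaled drag, then ignores movement until the next press.
; An interpolated move toward TargetPos is left unconnected.
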(event `self.ReceiveBeginPlay`
  (bind _returnvalue (pcsubsystem `EnhancedInputLocalPlayerSubsystem` (`GameplayStatics.GetPlayerController` 0)))
  ;[0.849 0.8382 0.001043 0.5] Input
  (`EnhancedInputSubsystemInterface.AddMappingContext` _returnvalue "/Game/Input/IMC_Default.IMC_Default" 0 (struct))
  (`EnhancedInputSubsystemInterface.AddMappingContext` _returnvalue "/Game/Input/IMC_NightControls.IMC_NightControls" 0 (struct)))

(event `EnhancedInput|/Game/Input/Actions/IA_Move`
  (params (ActionValue :type "Vector2D Structure") (ElapsedSeconds :type "Float (double-precision)") (TriggeredSeconds :type "Float (double-precision)") (InputAction :type "InputAction Object Reference" :default "/Game/Input/Actions/IA_Move.IA_Move"))
  (:`Triggered`
    (`self.AddMovementInput` (`KismetMathLibrary.GetForwardVector` (`self.K2_GetActorRotation`)) ActionValue_Y)
    (`self.AddMovementInput` (`KismetMathLibrary.GetRightVector` (`self.K2_GetActorRotation`)) ActionValue_X)))

(event `EnhancedInput|/Game/Input/Actions/IA_TouchDrag`
  (params (ActionValue :type "Vector2D Structure") (ElapsedSeconds :type "Float (double-precision)") (TriggeredSeconds :type "Float (double-precision)") (InputAction :type "InputAction Object Reference" :default "/Game/Input/Actions/IA_TouchDrag.IA_TouchDrag")))

(event `InputTouch`
  (params (Location :type "Vector Structure") (FingerIndex :type "ETouchIndex Enum"))
  (bind _returnvalue (`KismetMathLibrary.MakeVector2D` Location_X Location_Y))
  (bind (_returnvalue_x _returnvalue_y) (`KismetMathLibrary.BreakVector2D` (- (`self.TouchStartPos`) (`self.TouchCurrentPos`))))
  (bind (_returnvalue_x_2 _returnvalue_y_2) (`KismetMathLibrary.BreakVector2D` (- (`self.TouchStartPos`) (`self.TouchCurrentPos`))))
  (bind _returnvalue_x_3 (`KismetMathLibrary.BreakVector2D` (- (`self.TouchStartPos`) (`self.TouchCurrentPos`))))
  (bind _returnvalue_x_4 (`KismetMathLibrary.BreakVector2D` (- (`self.TouchStartPos`) (`self.TouchCurrentPos`))))
  (:`Pressed`
    (set `self.TouchStartPos` _returnvalue)
    (set `self.TouchActive` true))
  (:`Released`
    (set `self.TouchActive` false))
  (:`Moved`
    (set `self.TouchCurrentPos` _returnvalue)
    (if (`self.TouchActive`)
      (`|ExecutionSequence`
        (:`then_0`
          (if (> _returnvalue_x_3 (`self.TouchMoveThreshold`))
            (set `self.TouchActive` false)
            (`KismetSystemLibrary.PrintString` "Left")
            (`self.K2_AddActorWorldOffset` (`KismetMathLibrary.MakeVector` (* _returnvalue_x_3 3.0)))))
        (:`then_1`
          (if (< _returnvalue_x_4 (* (`self.TouchMoveThreshold`) -1.0))
            (set `self.TouchActive` false)
            (`KismetSystemLibrary.PrintString` "Right")
            (`self.K2_AddActorWorldOffset` (`KismetMathLibrary.MakeVector` (* _returnvalue_x_4 3.0)))))
        (:`then_2`
          (if (> _returnvalue_y_2 (`self.TouchMoveThreshold`))
            (set `self.TouchActive` false)
            (`KismetSystemLibrary.PrintString` "Up")
            (`self.K2_AddActorWorldOffset` (`KismetMathLibrary.MakeVector` 0.0 (* _returnvalue_y_2 3.0)))))
        (:`then_3`
          (if (< _returnvalue_y (* (`self.TouchMoveThreshold`) -1.0))
            (set `self.TouchActive` false)
            (`KismetSystemLibrary.PrintString` "Down")
            (`self.K2_AddActorWorldOffset` (`KismetMathLibrary.MakeVector` 0.0 (* _returnvalue_y 3.0)))))))))

(event `self.ReceiveTick`
  (params (DeltaSeconds :type "Float (single-precision)")))

(fn `UserConstructionScript`)