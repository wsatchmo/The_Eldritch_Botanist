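; BP_PlantDataStore holds the data of one plant for use by the spawner.
; Its UpdatePlantData event copies the passed button instance, identity, level, stats, build cost, display info and actor class into its own variables, then sets CanSummon to true.
; The Blueprint only stores state and contains no spawning logic, and its construction script is empty.
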(event `UpdatePlantData`
  (params (ButtonInstance :type "/Game/_Blueprints/UI/NightUI/UMG_GreenhouseItemNight Object Reference") (PlantID :type "/Game/_Blueprints/Data/E_PlantID Enum" :default "NewEnumerator11") (PlantLevel :type Integer) (name :type String) (Health :type Integer) (Attack :type Integer) (AttackSpeed :type "Float (double-precision)") (BuildCost :type Integer) (Icon :type "Texture2D Object Reference") (Info :type String) (ActorClass :type "/Game/_Blueprints/Character/Plants/BP_PlantBase Class Reference"))
  ;[0 0 0] Store data for Spawner
  (set `self.ButtonInstance` ButtonInstance)
  (set `self.PlantID` PlantID)
  (set `self.Level` PlantLevel)
  (set `self.Name` name)
  (set `self.Health` Health)
  (set `self.Attack` Attack)
  (set `self.Attack Speed` AttackSpeed)
  (set `self.Build Cost` BuildCost)
  (set `self.Icon` Icon)
  (set `self.Info` Info)
  (set `self.ActorClass` ActorClass)
  (set `self.CanSummon` true))

(fn `UserConstructionScript`)