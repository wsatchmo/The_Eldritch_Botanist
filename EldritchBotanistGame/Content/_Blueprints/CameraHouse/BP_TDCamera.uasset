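; Top-down touch camera that pans on XY with a one-finger swipe and zooms along Z with a two-finger pinch.
; Touch events set targets, clamped by BP_CameraBounds for pan and min/max height for zoom, which Tick interpolates toward while fingers are down.
; A timer-reset flag suppresses swiping after a pinch.
; Game instance settings set initial inversion, but InvertScroll flips ZoomLogic and InvertZoom flips ScrollLogic.
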(event `self.ReceiveBeginPlay`
  (bind (_returnvalue_x _returnvalue_y _returnvalue_z) (`KismetMathLibrary.BreakVector` (`self.K2_GetActorLocation`)))
  (bind _returnvalue (pcsubsystem `EnhancedInputLocalPlayerSubsystem` (`GameplayStatics.GetPlayerController` 0)))
  ;[0.849 0.8382 0.001043 0.5] Input
  (`EnhancedInputSubsystemInterface.AddMappingContext` _returnvalue "/Game/Input/IMC_Default.IMC_Default" 0 (struct))
  (`EnhancedInputSubsystemInterface.AddMappingContext` _returnvalue "/Game/Input/IMC_NightControls.IMC_NightControls" 0 (struct))
  ;[0 0 0 0.5] Cam Location set
  (set `self.CamTargetPos` (`KismetMathLibrary.Conv_VectorToVector2D` (`KismetMathLibrary.MakeVector` _returnvalue_x _returnvalue_y)))
  (set `self.CurrentZ` _returnvalue_z)
  (bind _asbp_tebgame_instance (cast `/Game/_Blueprints/InstanceAndSave/BP_TEBGameInstance` (`GameplayStatics.GetGameInstance`)))
  (`|ExecutionSequence`
    (:`then_0`
      (if (`/Game/_Blueprints/InstanceAndSave/BP_TEBGameInstance.InvertScroll?` _asbp_tebgame_instance)
        (set `self.ScrollLogic` 1.0)
        (else
          (set `self.ScrollLogic` -1.0))))
    (:`then_1`
      (if (`/Game/_Blueprints/InstanceAndSave/BP_TEBGameInstance.InvertZoom?` _asbp_tebgame_instance)
        (set `self.ZoomLogic` -1.0)
        (else
          (set `self.ZoomLogic` 1.0)))))
  ; (Wait .02 seconds to load the camera bounds actor)
  (`KismetSystemLibrary.Delay` 0.2)
  ;[0 0 0 0.5] Camera bounds ref
  (bind _returnvalue_2 (`GameplayStatics.GetActorOfClass` "/Game/_Blueprints/CameraHouse/BP_CameraBounds.BP_CameraBounds_C"))
  (set `self.CameraBoundsRef` _returnvalue_2))

(event `InputTouch`
  (params (Location :type "Vector Structure") (FingerIndex :type "ETouchIndex Enum"))
  (bind _returnvalue (`KismetMathLibrary.MakeVector2D` Location_X Location_Y))
  (bind _pinchresethandle (`self.PinchResetHandle`))
  (bind _returnvalue_2 (`KismetMathLibrary.Distance2D` (`self.Touch1Pos`) (`self.Touch2Pos`)))
  (bind _returnvalue_3 (- _returnvalue_2 (`self.LastPinchDistance`)))
  (bind (_returnvalue_x _returnvalue_y) (`KismetMathLibrary.BreakVector` (+ (`self.K2_GetActorLocation`) (* (- (`self.TouchCurrentPos`) (`self.TouchLastPos`)) (`self.ScrollSpeed`) (`self.ScrollLogic`)))))
  ;[0.7823 0.5388 0 0.5] Touch movement
  (:`Pressed`
    (bind _output_get (set `self.TouchCurrentPos` _returnvalue))
    (set `self.TouchLastPos` _output_get)
    (set `self.TouchActive` true)
    (bind _output_get_2 (set `self.ActiveTouchCount` (+ (`self.ActiveTouchCount`) 1)))
    (if (== _output_get_2 2)
      (set `self.LastPinchDistance` (`KismetMathLibrary.Distance2D` (`self.Touch1Pos`) (`self.Touch2Pos`)))
      (set `self.PinchStartFrame?` true)))
  (:`Released`
    (bind _output_get_3 (set `self.ActiveTouchCount` (- (`self.ActiveTouchCount`) 1)))
    (if (!= _output_get_3 1)
      (set `self.TouchLastPos` (`self.TouchCurrentPos`))
      (if (<= _output_get_3 0)
        (set `self.TouchActive` false)
        (set `self.ActiveTouchCount` 0)
        (`KismetSystemLibrary.K2_ClearAndInvalidateTimerHandle` (`self.PinchResetHandle`))
        (set `self.RecentlyZoomed?` false))))
  (:`Moved`
    (set `self.TouchCurrentPos` _returnvalue)
    (switch `ETouchIndex` FingerIndex
      (:`Touch1`
        (set `self.Touch1Pos` _returnvalue))
      (:`Touch2`
        (set `self.Touch2Pos` _returnvalue)))
    (if (`self.TouchActive`)
      (switch `int` (`self.ActiveTouchCount`) ; 0: Do nothing\n1: Swipe Logic\n2: Pinch Logic\nDefault: Do nothing
        (:`1`
          ;;[1 0.9809 0 0.5] SWIPE LOGIC
          (if (`KismetSystemLibrary.K2_IsValidTimerHandle` _pinchresethandle)
            (`KismetSystemLibrary.K2_ClearAndInvalidateTimerHandle` _pinchresethandle))
          (`self.ResetPinchTimer`)
          (if (not (`self.RecentlyZoomed?`))
            (bind _clampedlocation (`/Game/_Blueprints/CameraHouse/BP_CameraBounds.ClampLocation` (`self.CameraBoundsRef`) (`KismetMathLibrary.MakeVector` _returnvalue_x _returnvalue_y)))
            (set `self.CamTargetPos` (`KismetMathLibrary.MakeVector2D` (.x _clampedlocation) (.y _clampedlocation)))
            (set `self.TouchLastPos` (`self.TouchCurrentPos`)) ; DISCONNECT:\nMore stable, movement  constrained to vector\nCONNECT: \nStable, free movement
          ))
        (:`2`
          (if (`self.PinchStartFrame?`)
            (set `self.PinchStartFrame?` false)
            (else
              ;;[1 0.9809 0 0.5] PINCH LOGIC
              (set `self.RecentlyZoomed?` true)
              (if (< _returnvalue_3 (`self.ZoomInThreshold`))
                (set `self.CurrentZ` (`KismetMathLibrary.FClamp` (- (`self.CurrentZ`) (* _returnvalue_3 (`self.ZoomSpeed`) (`self.ZoomLogic`))) (`self.MinZoomZ`) (`self.MaxZoomZ`)))
                (set `self.LastPinchDistance` _returnvalue_2)))))))))

(event `self.ReceiveTick`
  (params (DeltaSeconds :type "Float (single-precision)"))
  (bind (_returnvalue_x _returnvalue_y _returnvalue_z) (`KismetMathLibrary.BreakVector` (`self.K2_GetActorLocation`)))
  (bind _currentz (`self.CurrentZ`))
  (bind (_x _y) (`KismetMathLibrary.BreakVector2D` (`self.CamTargetPos`)))
  (bind (_x_2 _y_2) (`KismetMathLibrary.BreakVector2D` (`self.CamTargetPos`)))
  (bind (_x_3 _y_3) (`KismetMathLibrary.BreakVector2D` (`KismetMathLibrary.Conv_VectorToVector2D` (`self.K2_GetActorLocation`))))
  (bind (_returnvalue_x_2 _returnvalue_y_2 _returnvalue_z_2) (`KismetMathLibrary.BreakVector` (`KismetMathLibrary.VInterpTo` (`KismetMathLibrary.MakeVector` _x_3 _y_3 _currentz) (`KismetMathLibrary.MakeVector` _x_2 _y_2 _currentz) DeltaSeconds (`self.ScrollInterpSpeed`))))
  ;[1 0.8793 0 0.5] Touch control Tick
  (switch `int` (`self.ActiveTouchCount`) ; 0: Do nothing\n1: Swipe Logic\n2: Pinch Logic\nDefault: Do nothing
    (:`1`
      (`self.K2_SetActorLocation` (`KismetMathLibrary.MakeVector` _returnvalue_x_2 _returnvalue_y_2 _returnvalue_z_2)))
    (:`2`
      (`self.K2_SetActorLocation` (`KismetMathLibrary.MakeVector` _x _y (`KismetMathLibrary.FInterpTo` _returnvalue_z (`self.CurrentZ`) DeltaSeconds (`self.ZoomInterpSpeed`)))))))

(fn `InvertScroll`
  (if (== (`self.ZoomLogic`) 1.0)
    (set `self.ZoomLogic` -1.0)
    (else
      (set `self.ZoomLogic` 1.0))))

(fn `InvertZoom`
  (if (== (`self.ScrollLogic`) 1.0)
    (set `self.ScrollLogic` -1.0)
    (else
      (set `self.ScrollLogic` 1.0))))

(fn `ResetPinch`
  (set `self.RecentlyZoomed?` false))

(fn `ResetPinchTimer`
  (bind _returnvalue (`KismetSystemLibrary.K2_SetTimer` null "ResetPinch" 0.8))
  (set `self.PinchResetHandle` _returnvalue))

(fn `UserConstructionScript`)