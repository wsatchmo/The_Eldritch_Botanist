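; BP_CameraBounds is a Blueprint that defines a volume for limiting a location, apparently the camera's, to a horizontal area.
; ClampLocation takes the Bounds component's world-space origin and extent to get its minimum and maximum corners.
; It clamps the input X and Y to that axis-aligned range and returns the vector with Z unchanged.
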(fn `ClampLocation`
  (params (Location :type "Vector Structure"))
  (returns (ClampedLocation :type "Vector Structure"))
  (bind (_origin _boxextent) (`KismetSystemLibrary.GetComponentBounds` (`self.Bounds`)))
  (return (`KismetMathLibrary.MakeVector` (`KismetMathLibrary.FClamp` (.x (`KismetMathLibrary.MakeVector` Location_X Location_Y Location_Z)) (.x (- _origin _boxextent)) (.x (+ _origin _boxextent))) (`KismetMathLibrary.FClamp` (.y (`KismetMathLibrary.MakeVector` Location_X Location_Y Location_Z)) (.y (- _origin _boxextent)) (.y (+ _origin _boxextent))) Location_Z)))

(fn `UserConstructionScript`)