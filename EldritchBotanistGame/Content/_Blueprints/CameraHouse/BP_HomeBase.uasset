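; BP_HomeBase is the night-defense level manager and house that loses health when enemies reach its collision box, opening Game_Over at zero.
; It loads the selected level from DT_LevelData, splits enemies into waves across BP_EnemySpawners when randomized, and drives start and between-wave countdown widgets with pausable timers.
; When all enemies are gone, it upgrades matching inventory plants, grants random rewards, saves, and shows the finish screen.
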(event `PauseSpawnTimer`
  (bind _wavetimerref (`self.WaveTimerRef`))
  (bind _wavetimerref_2 (`self.WaveTimerRef`))
  ;[0.03835 0.01618 0.15 0.5] Handling pause/unpause for spawn timer and wave countdown timer
  (if (`self.SpawnTimerPaused?`)
    (`KismetSystemLibrary.K2_UnPauseTimerHandle` (`self.StarterHandleRef`))
    (set `/Game/_Blueprints/Character/Spawners/WBP_LevelStart.IsUnpaused` true (`self.WBPLevelStartRef`))
    (set `self.SpawnTimerPaused?` false)
    (`KismetSystemLibrary.K2_UnPauseTimerHandle` (`self.WaveTimerHandle`))
    (`/Engine/EditorBlueprintResources/StandardMacros.IsValid` _wavetimerref_2
      (:`Is Valid`
        (set `/Game/_Blueprints/UI/NightUI/WBP_WaveTimer.IsUnpaused` true _wavetimerref_2)
        (set `self.WaveTimerWidgetPaused?` false)))
    (else
      (`KismetSystemLibrary.K2_PauseTimerHandle` (`self.StarterHandleRef`))
      (set `/Game/_Blueprints/Character/Spawners/WBP_LevelStart.IsUnpaused` false (`self.WBPLevelStartRef`))
      (set `self.SpawnTimerPaused?` true)
      (`KismetSystemLibrary.K2_PauseTimerHandle` (`self.WaveTimerHandle`))
      (`/Engine/EditorBlueprintResources/StandardMacros.IsValid` _wavetimerref
        (:`Is Valid`
          (set `/Game/_Blueprints/UI/NightUI/WBP_WaveTimer.IsUnpaused` false _wavetimerref)
          (set `self.WaveTimerWidgetPaused?` true))))))

(event `self.ReceiveBeginPlay`
  (bind _nightwidget_ref (`self.NightWidget_Ref`))
  (bind _maxtotalenemies (`self.MaxTotalEnemies`))
  (bind _start_delay (`self.Start Delay`))
  ;[0 0 0 0.5] Creat night widget & set Game Instance ref among other references
  (bind _returnvalue (`GameplayStatics.GetActorOfClass` "/Game/_Blueprints/Inventory/BP_PlantDataStore.BP_PlantDataStore_C"))
  (bind _asbp_plant_data_store (cast `/Game/_Blueprints/Inventory/BP_PlantDataStore` _returnvalue))
  (set `self.DataStoreRef` _asbp_plant_data_store)
  (bind _returnvalue_2 (`|CreateWidget` "/Game/_Blueprints/UI/NightUI/UMG_Greenhouse_Night.UMG_Greenhouse_Night_C" null null null))
  (`UserWidget.AddToViewport` _returnvalue_2 0)
  (set `self.NightWidget_Ref` _returnvalue_2)
  (bind _asbp_tebgame_instance (cast `/Game/_Blueprints/InstanceAndSave/BP_TEBGameInstance` (`GameplayStatics.GetGameInstance`)))
  (set `self.GameInstanceRef` _asbp_tebgame_instance)
  ;[0.7156 0.7062 0 0.5] Spawner Construction
  (`self.SpawnerSetup`)
  (bind _maxhealth (`/Game/_Blueprints/InstanceAndSave/BP_TEBGameInstance.MaxHealth` _asbp_tebgame_instance))
  ;[0.0358 0.0255 0.3823 0.5] Night Widget ref & setting text
  (bind _output_get (set `self.HouseHealth` _maxhealth))
  (`/Game/_Blueprints/UI/NightUI/UMG_Greenhouse_Night.SetHouseHealth` _returnvalue_2 _maxhealth _output_get)
  (`/Game/_Blueprints/UI/NightUI/UMG_Greenhouse_Night.SetEnemiesRemainingText` _nightwidget_ref _maxtotalenemies)
  (`/Game/_Blueprints/UI/NightUI/UMG_Greenhouse_Night.SetWaveText` _nightwidget_ref (`self.CurrentWave`) (`self.TotalWaves`))
  (set `self.CurrentTotalEnemies` _maxtotalenemies)
  ;[0.07877 0.0299 0.4823 0.5] Create the level start widget
  (bind _returnvalue_3 (`|CreateWidget` "/Game/_Blueprints/Character/Spawners/WBP_LevelStart.WBP_LevelStart_C" (`GameplayStatics.GetPlayerController` 0)))
  (bind _output_get_2 (set `self.WBPLevelStartRef` _returnvalue_3))
  (`UserWidget.AddToViewport` _output_get_2 0)
  (bind _aswbp_level_start (cast `/Game/_Blueprints/Character/Spawners/WBP_LevelStart` _output_get_2))
  ;[0.2551 0.09313 0.349 0.5] Bind start to the timer and the button
  (add `Button.OnClicked` (`/Game/_Blueprints/Character/Spawners/WBP_LevelStart.StartLevelButton` _aswbp_level_start) (delegate `StartWaves`))
  (set `/Game/_Blueprints/Character/Spawners/WBP_LevelStart.StartDelayTime` _start_delay _aswbp_level_start)
  (bind _returnvalue_4 (`KismetSystemLibrary.K2_SetTimerDelegate` (delegate `StartWaves`) _start_delay))
  (set `self.StarterHandleRef` _returnvalue_4)
  (set `self.SpawnTimerPaused?` false)
  ;[0.01106 0.0169 0.15 0.5] Start night tutorial iff it hast been seen yet
  (if (not (`/Game/_Blueprints/InstanceAndSave/BP_TEBGameInstance.NightTutorialComplete?` (`self.GameInstanceRef`)))
    (bind _returnvalue_5 (`|CreateWidget` "/Game/_Blueprints/UI/TutorialUI/WBP_NightTutorialPopup.WBP_NightTutorialPopup_C"))
    (`UserWidget.AddToViewport` _returnvalue_5 0)
    (`self.PauseSpawnTimer`) ; DON'T MOVE TO POPUP
  ))

(event `StartWaves`
  (bind _wbplevelstartref (`self.WBPLevelStartRef`))
  ;[0.1946 0.072 0.4713 0.5] Start all spawners and remove the WBP from the screen
  (`KismetSystemLibrary.K2_ClearAndInvalidateTimerHandle` (`self.StarterHandleRef`))
  (`self.StartNextWave`)
  (`Widget.RemoveFromParent` _wbplevelstartref)
  (clear `Button.OnClicked` (`/Game/_Blueprints/Character/Spawners/WBP_LevelStart.StartLevelButton` _wbplevelstartref)))

(event `self.Enemy_Collision_Box.OnComponentBeginOverlap`
  (params (OverlappedComponent :type "PrimitiveComponent Object Reference") (OtherActor :type "Actor Object Reference") (OtherComp :type "PrimitiveComponent Object Reference") (OtherBodyIndex :type Integer) (bFromSweep :type Boolean) (SweepResult :type "HitResult Structure (by ref)"))
  ;[0.008762 0.3365 0.0233 0.5] On enemy collision
  (bind _asbp_enemy_base (cast `/Game/_Blueprints/Character/Enemies/BP_EnemyBase` OtherActor))
  (`self.K2_DestroyActor` _asbp_enemy_base)
  (bind _output_get (set `self.HouseHealth` (- (`self.HouseHealth`) 1)))
  (if (<= _output_get 0)
    (`GameplayStatics.OpenLevel` "Game_Over")
    (else
      (`/Game/_Blueprints/UI/NightUI/UMG_Greenhouse_Night.SetHouseHealth` (`self.NightWidget_Ref`) (`/Game/_Blueprints/InstanceAndSave/BP_TEBGameInstance.MaxHealth` (`self.GameInstanceRef`)) (`self.HouseHealth`))
      (`self.OnEnemyDeath`))))

(event `OnEnemyDeath`
  ;[0.424 0 0 0.5] Enemy Death
  (bind _output_get (set `self.CurrentTotalEnemies` (- (`self.CurrentTotalEnemies`) 1)))
  (`/Game/_Blueprints/UI/NightUI/UMG_Greenhouse_Night.SetEnemiesRemainingText` (`self.NightWidget_Ref`) _output_get)
  (if (<= _output_get 0)
    ;[1 1 1 0.5 40] Player Victory
    (`self.PlayerVictory`)
    (else
      ;[0.15 0.1096 0.01465 0.5] Reduce wave & check if clear
      (bind _output_get_2 (set `self.RemainingThisWave` (- (`self.RemainingThisWave`) 1)))
      (if (<= _output_get_2 0)
        (`self.OnWaveCleared`)))))

(event `OnCountdownTick`
  ;[0.0618 0.15 0.02973 0.5] Wave countdown
  (bind _output_get (set `self.TimerTemp` (- (`self.TimerTemp`) 1.0)))
  (if (<= _output_get (`self.WarningTime`))
    (if (not (`self.WaveTimerWidgetEnabled?`))
      (set `self.WaveTimerWidgetEnabled?` true)
      ;;[0.05443 0.07951 0.599 0.5] Create / update countdown widget
      (bind _returnvalue (`|CreateWidget` "/Game/_Blueprints/UI/NightUI/WBP_WaveTimer.WBP_WaveTimer_C"))
      (bind _output_get_2 (set `self.WaveTimerRef` _returnvalue))
      (`UserWidget.AddToViewport` _output_get_2 0)
      (add `Button.OnClicked` (`/Game/_Blueprints/UI/NightUI/WBP_WaveTimer.WaveStartButton` _output_get_2) (delegate `EndWaveCountdown`)))
    (`RichTextBlock.SetText` (`/Game/_Blueprints/UI/NightUI/WBP_WaveTimer.WaveStartTimer` (`self.WaveTimerRef`)) (`KismetTextLibrary.Conv_DoubleToText` _output_get "HalfToEven")))
  (if (<= (`self.TimerTemp`) 0.0)
    (`self.EndWaveCountdown`)))

(event `EndWaveCountdown`
  ;[0.07956 0.2031 0.03214 0.5] Starting Next Wave
  (`Widget.RemoveFromParent` (`self.WaveTimerRef`))
  (`KismetSystemLibrary.K2_ClearAndInvalidateTimerHandle` (`self.WaveTimerHandle`))
  (`self.StartNextWave`))

(fn `OnWaveCleared`
  (set `self.WaveInProgress?` false)
  (set `self.TimerTemp` (`self.Time Between Waves`))
  (bind _returnvalue (`KismetSystemLibrary.K2_SetTimer` null "OnCountdownTick" 1.0 true))
  (set `self.WaveTimerHandle` _returnvalue))

(fn `PlayerVictory`
  (`self.UpgradePlants`)
  (`self.RewardRandomLoot`))

(fn `RandomizeRewards`
  (params (PossibleRewards :type "Array of /Game/_Blueprints/Data/e_ResourceID Enum"))
  (locals (PossRewards :type "Array of /Game/_Blueprints/Data/e_ResourceID Enum"))
  (bind _output_get (set `local.PossRewards` PossibleRewards))
  (for _ (range 1 (+ (`self.RewardAmt`) 1))
    (`KismetArrayLibrary.Array_Add` (`self.RewardsToBeGiven`) (`KismetArrayLibrary.Array_Random` _output_get))))

(fn `RewardRandomLoot`
  (bind _resourcesgivenmap (`self.ResourcesGivenMap`))
  (bind _rewardstobegiven (`self.RewardsToBeGiven`))
  (bind _mapindex (`self.MapIndex`))
  (bind _returnvalue (+ _mapindex 1))
  ;[0.1179 0.01907 0.15 0.5] Give player random items from possible items to earn
  (for _array_element _rewardstobegiven
    (bind (_str_inventoryslot_planttype _str_inventoryslot_resourcetype _str_inventoryslot_level) (break `/Game/_Blueprints/Data/STR_InventorySlot` (make `/Game/_Blueprints/Data/STR_InventorySlot` "NewEnumerator11" _array_element 0)))
    (`/Game/_Blueprints/InstanceAndSave/BP_TEBGameInstance.AddItem` (`self.GameInstanceRef`) "NewEnumerator11" _str_inventoryslot_resourcetype _str_inventoryslot_level))
  (`/Game/_Blueprints/InstanceAndSave/BP_TEBGameInstance.SaveGameInstance` (`self.GameInstanceRef`))
  (for _array_element_2 _rewardstobegiven
    (bind _outrownames (`DataTableFunctionLibrary.GetDataTableRowNames` "/Game/_Blueprints/Data/DT_ItemRegistry.DT_ItemRegistry"))
    (for _array_element_3 _outrownames
      (bind _returnvalue_2 (`|GetDataTableRow` "/Game/_Blueprints/Data/DT_ItemRegistry.DT_ItemRegistry" _array_element_3)
        (:`then`
          (bind (_isplant _plantid _isresource _resourceid _name) (break `/Game/_Blueprints/Data/STR_UnitData` _returnvalue_2))
          (if (`|EnumEquality` _resourceid _array_element_2)
            (`KismetArrayLibrary.Array_Add` (`self.ResourcesGivenNames`) _name))))))
  (for _array_element_4 (`self.ResourcesGivenNames`)
    (bind (_value _returnvalue_3) (`BlueprintMapLibrary.Map_Find` _resourcesgivenmap _array_element_4))
    (if _returnvalue_3
      (`BlueprintMapLibrary.Map_Add` _resourcesgivenmap _array_element_4 (+ _value 1))
      (else
        (`BlueprintMapLibrary.Map_Add` _resourcesgivenmap _array_element_4 1))))
  (bind (_keypin _valuepin) (`|MapForEach` (`self.ResourcesGivenMap`))
    (:`then`
      (if (== _mapindex 0)
        (set `self.Rewards Statement` (`KismetStringLibrary.Concat_StrStr` (`KismetStringLibrary.Conv_IntToString` _valuepin) " " _keypin))
        (set `self.MapIndex` _returnvalue)
        (else
          (set `self.Rewards Statement` (`KismetStringLibrary.Concat_StrStr` (`self.Rewards Statement`) ", " (`KismetStringLibrary.Conv_IntToString` _valuepin) " " _keypin))
          (set `self.MapIndex` _returnvalue))))
    (:`CompletedPin`
      (`GameplayStatics.SetGamePaused` true)
      (bind _returnvalue_4 (`|CreateWidget` "/Game/_Blueprints/UI/MenusUI/WBP_LevelFinishUI.WBP_LevelFinishUI_C" (`GameplayStatics.GetPlayerController` 0)))
      (`TextBlock.SetText` (`/Game/_Blueprints/UI/MenusUI/WBP_LevelFinishUI.RewardsText` _returnvalue_4) (`KismetTextLibrary.Conv_StringToText` (`self.Rewards Statement`)))
      (`UserWidget.AddToViewport` _returnvalue_4 0))))

(fn `SpawnerSetup`
  (locals (SpawnerCount :type Integer :default 0) (BaseAmt :type Integer) (UnitRemainder :type Integer :default 0))
  (bind _outrownames (`DataTableFunctionLibrary.GetDataTableRowNames` "/Game/_Blueprints/Data/DT_LevelData.DT_LevelData"))
  (for _array_element _outrownames
    (bind _returnvalue (`|GetDataTableRow` "/Game/_Blueprints/Data/DT_LevelData.DT_LevelData" _array_element)
      (:`then`
        (bind (_levelbyitem _levelname _leveltitle _totalenemies _waves _timebetweenwaves _wavewarningtime _startdelay _enemytypes _possiblerewards _rewardsamt _israndom_ _exp) (break `/Game/_Blueprints/Data/STR_LevelItem` _returnvalue))
        (if (`|EnumEquality` (`/Game/_Blueprints/InstanceAndSave/BP_TEBGameInstance.SelectedLevel` (`self.GameInstanceRef`)) _levelbyitem)
          (set `self.MaxTotalEnemies` _totalenemies)
          (set `self.TotalWaves` _waves)
          (set `self.EnemiesPerWave` (/ _totalenemies _waves))
          (set `self.RemainderEnemies` (mod _totalenemies _waves))
          (set `self.CurrentWave` 0)
          (set `self.Time Between Waves` _timebetweenwaves)
          (set `self.WarningTime` _wavewarningtime)
          (set `self.Start Delay` _startdelay)
          (set `self.SpawnableTypes` _enemytypes)
          (bind _output_get (set `self.PossibleRewards` _possiblerewards))
          (set `self.RewardAmt` _rewardsamt)
          (set `self.Is Randomized?` _israndom_)
          (set `self.ExpGainOnComplete` _exp)
          (`self.RandomizeRewards` _output_get))))))

(fn `SpawnHandler`
  (params (TotalThisWave :type Integer))
  (locals (SpawnerCount :type Integer) (EnemiesPerSpawner :type Integer) (UnitRemainder :type Integer))
  (if (`self.Is Randomized?`)
    (bind _outactors (`GameplayStatics.GetAllActorsOfClass` "/Game/_Blueprints/Character/Spawners/BP_EnemySpawner.BP_EnemySpawner_C"))
    (bind _returnvalue (`KismetArrayLibrary.Array_Length` _outactors))
    (set `local.SpawnerCount` _returnvalue)
    (bind _output_get (set `local.EnemiesPerSpawner` (/ TotalThisWave _returnvalue)))
    (bind _output_get_2 (set `local.UnitRemainder` (mod TotalThisWave _returnvalue)))
    (for (_array_element _array_index) _outactors
      (set `/Game/_Blueprints/Character/Spawners/BP_EnemySpawner.AmtSpawned` 0 _array_element)
      (bind _output_get_3 (set `/Game/_Blueprints/Character/Spawners/BP_EnemySpawner.AmtToSpawn` _output_get _array_element))
      (set `/Game/_Blueprints/Character/Spawners/BP_EnemySpawner.TypesToSpawn` (`self.SpawnableTypes`) _array_element)
      (if (< _array_index _output_get_2)
        (set `/Game/_Blueprints/Character/Spawners/BP_EnemySpawner.AmtToSpawn` (+ _output_get_3 1) _array_element))
      (`/Game/_Blueprints/Character/Spawners/BP_EnemySpawner.SetSpawnerTimer` _array_element))))

(fn `StartNextWave`
  (if (<= (`self.CurrentWave`) (`self.TotalWaves`))
    (bind _output_get (set `self.CurrentWave` (+ (`self.CurrentWave`) 1)))
    (`/Game/_Blueprints/UI/NightUI/UMG_Greenhouse_Night.SetWaveText` (`self.NightWidget_Ref`) _output_get (`self.TotalWaves`))
    (set `self.WaveInProgress?` true)
    (bind _output_get_2 (set `self.RemainingThisWave` (`self.EnemiesPerWave`)))
    (if (== (`self.CurrentWave`) (`self.TotalWaves`))
      (set `self.RemainingThisWave` (+ _output_get_2 (`self.RemainderEnemies`))))
    (`self.SpawnHandler` (`self.RemainingThisWave`))))

(fn `UpgradePlants`
  (bind _inventoryitems (`/Game/_Blueprints/InstanceAndSave/BP_TEBGameInstance.InventoryItems` (`self.GameInstanceRef`)))
  ;[0.08567 0.03466 0.15 0.5] Check used items against inventory array items, only if the plant is below level 3
  (for _array_element (`/Game/_Blueprints/Inventory/BP_PlantDataStore.SpawnedPlantsArr` (`self.DataStoreRef`))
    (if (not (>= (`.SpawnedPlantLevel_6_48A4DDFF411295BF2E6E8B94E0577E47` (break `/Game/_Blueprints/Inventory/STR_SpawnedPlant` _array_element)) 3))
      (for (_array_element_2 _array_index) (`/Game/_Blueprints/InstanceAndSave/BP_TEBGameInstance.InventoryItems` (`self.GameInstanceRef`))
        (if (`|EnumEquality` (break `/Game/_Blueprints/Data/STR_InventorySlot` _array_element_2) (break `/Game/_Blueprints/Inventory/STR_SpawnedPlant` _array_element))
          (if (== (`.Level_18_9084E43249BB4C0CA2252789485B5E37` (break `/Game/_Blueprints/Data/STR_InventorySlot` _array_element_2)) (`.SpawnedPlantLevel_6_48A4DDFF411295BF2E6E8B94E0577E47` (break `/Game/_Blueprints/Inventory/STR_SpawnedPlant` _array_element)))
            (`KismetArrayLibrary.Array_Add` (`self.IndicesToKill`) _array_index)
            (`KismetArrayLibrary.Array_Add` (`/Game/_Blueprints/InstanceAndSave/BP_TEBGameInstance.InventoryItems` (`self.GameInstanceRef`)) (make `/Game/_Blueprints/Data/STR_InventorySlot` (break `/Game/_Blueprints/Data/STR_InventorySlot` _array_element_2) "NewEnumerator12" (+ (`.Level_18_9084E43249BB4C0CA2252789485B5E37` (break `/Game/_Blueprints/Data/STR_InventorySlot` _array_element_2)) 1))) ; Increase Level by 1 and add Plant to inventory
            (break))))))
  ;[0.06274 0.01983 0.15 0.5] Reverse for each loop to delete items from inventory
  (for _array_element_3 (`self.IndicesToKill`)
    (bind (_arrayindex _arrayelement) (`/Engine/EditorBlueprintResources/StandardMacros.ReverseForEachLoop` _inventoryitems)
      (:`LoopBody`
        (if (== _arrayindex _array_element_3)
          (`KismetArrayLibrary.Array_RemoveItem` _inventoryitems)))
      (:`Completed`
        (`/Game/_Blueprints/InstanceAndSave/BP_TEBGameInstance.SaveGameInstance` (`self.GameInstanceRef`))))))

(fn `UserConstructionScript`)