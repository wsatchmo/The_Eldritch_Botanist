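; Game instance Blueprint that holds the player's inventory as an array of slot structs with ID, quantity and level.
; AddItem appends a new slot; its stack-merging loop is left unwired.
; RemoveItem and GetQuantity match whole structs using fixed zero quantity, not ID alone.
; Save and load use the "SaveGame" slot, but neither transfers the inventory array, and the loaded object is discarded.
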(fn `AddItem`
  (params (ItemId :type Name) (Quantity :type Integer) (Level :type Integer))
  (`KismetArrayLibrary.Array_Add` (`self.InventoryItems`) (make `/Game/_Blueprints/Data/STR_InventorySlot` ItemId Quantity Level)))

(fn `GetQuantity`
  (params (ID :type Name))
  (returns (Quantity :type Integer))
  (bind _inventoryitems (`self.InventoryItems`))
  (bind (_output_id _output_quantity) (break `/Game/_Blueprints/Data/STR_InventorySlot` (`|GetArrayItem` _inventoryitems (`KismetArrayLibrary.Array_Find` _inventoryitems (make `/Game/_Blueprints/Data/STR_InventorySlot` ID)))))
  (return _output_quantity))

(fn `LoadInventory`
  (`GameplayStatics.LoadGameFromSlot` "SaveGame"))

(fn `RemoveItem`
  (params (ItemId :type Name) (Quantity :type Integer) (Level :type Integer))
  (`KismetArrayLibrary.Array_RemoveItem` (`self.InventoryItems`) (make `/Game/_Blueprints/Data/STR_InventorySlot` ItemId 0 Level)))

(fn `SaveInventory`
  (bind _asbp_save_game (cast `/Game/_Blueprints/InstanceAndSave/BP_SaveGame` (`self.SaveGame`)))
  (`GameplayStatics.SaveGameToSlot` _asbp_save_game "SaveGame"))