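; BP_HomeBase is the base enemies attack, deciding when the level is lost or finished.
; Enemies overlapping its collision box are counted, and reaching the maximum opens the Game_Over level.
; OnEnemyDeath counts kills: hitting the minimum starts a delayed EndLevel timer, while reaching the full enemy count cancels it and ends immediately.
; EndLevel shows the WBP_LevelFinishUI widget.
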(event `self.Enemy_Collision_Box.OnComponentBeginOverlap`
  (params (OverlappedComponent :type "PrimitiveComponent Object Reference") (OtherActor :type "Actor Object Reference") (OtherComp :type "PrimitiveComponent Object Reference") (OtherBodyIndex :type Integer) (bFromSweep :type Boolean) (SweepResult :type "HitResult Structure (by ref)"))
  (cast `/Game/_Blueprints/Character/Enemies/BP_EnemyBase` OtherActor)
  (`KismetSystemLibrary.PrintString` "Enemy Collided")
  (set `self.EnemyCollisions` (+ (`self.EnemyCollisions`) 1))
  (if (>= (`self.EnemyCollisions`) (`self.MaxEnemyCollisions`))
    (`GameplayStatics.OpenLevel` "Game_Over")))

(event `OnEnemyDeath`
  (set `self.EnemiesKilled` (+ (`self.EnemiesKilled`) 1))
  (`self.EnoughEnemiesKilled`)
  (`self.AllEnemiesKilled`))

(event `EnoughEnemiesKilled`
  (if (== (`self.EnemiesKilled`) (`self.MinEnemiesKilled`))
    (bind _returnvalue (`KismetSystemLibrary.K2_SetTimerDelegate` (delegate `EndLevel`) 33.0))
    (set `self.EndLevHandle` _returnvalue)))

(event `EndLevel`
  (bind _returnvalue (`|CreateWidget` "/Game/_Blueprints/UI/MenusUI/WBP_LevelFinishUI.WBP_LevelFinishUI_C" (`GameplayStatics.GetPlayerController` 0)))
  (`UserWidget.AddToViewport` _returnvalue 0))

(event `AllEnemiesKilled`
  (if (== (`self.EnemiesKilled`) (`self.EnemyAmt`))
    (`KismetSystemLibrary.K2_ClearAndInvalidateTimerHandle` (`self.EndLevHandle`))
    (`self.EndLevel`)))

(fn `UserConstructionScript`)