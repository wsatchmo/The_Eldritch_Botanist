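; Game instance that holds the player's inventory as an array of ID and quantity slots, with add, remove, quantity lookup and save/load functions.
; AddItem loops the slots, raising quantity on an ID match and appending a slot for each non-match.
; Removal and lookup match whole structs rather than IDs.
; Save writes the SaveGame object to a fixed slot without copying the inventory, and load discards its result.
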(fn `AddItem`
  (params (ItemId :type Name) (Quantity :type Integer))
  (bind _inventoryitems (`self.InventoryItems`))
  (for (_array_element _array_index) _inventoryitems
    (if (== (break `/Game/_Blueprints/DataAssets/STR_InventorySlot` _array_element) ItemId)
      (bind (_id _quantity) (break `/Game/_Blueprints/DataAssets/STR_InventorySlot` (make `/Game/_Blueprints/DataAssets/STR_InventorySlot` (break `/Game/_Blueprints/DataAssets/STR_InventorySlot` _array_element) (+ Quantity (`.Quantity_6_B667766346A026D4622E9B8CF4C9BB8C` (break `/Game/_Blueprints/DataAssets/STR_InventorySlot` _array_element))))))
      (`KismetArrayLibrary.Array_Set` (`self.InventoryItems`) _array_index (make `/Game/_Blueprints/DataAssets/STR_InventorySlot` _id _quantity))
      (else
        (`KismetArrayLibrary.Array_Add` _inventoryitems (make `/Game/_Blueprints/DataAssets/STR_InventorySlot` ItemId Quantity))))))

(fn `GetQuantity`
  (params (ID :type Name))
  (returns (Quantity :type Integer))
  (bind _inventoryitems (`self.InventoryItems`))
  (bind (_output_id _output_quantity) (break `/Game/_Blueprints/DataAssets/STR_InventorySlot` (`|GetArrayItem` _inventoryitems (`KismetArrayLibrary.Array_Find` _inventoryitems (make `/Game/_Blueprints/DataAssets/STR_InventorySlot` ID)))))
  (return _output_quantity))

(fn `LoadInventory`
  (`GameplayStatics.LoadGameFromSlot` "SaveGame"))

(fn `RemoveItem`
  (params (ItemId :type Name) (Quantity :type Integer))
  (`KismetArrayLibrary.Array_RemoveItem` (`self.InventoryItems`) (make `/Game/_Blueprints/DataAssets/STR_InventorySlot` ItemId Quantity)))

(fn `SaveInventory`
  (bind _asbp_save_game (cast `/Game/_Blueprints/DataAssets/BP_SaveGame` (`self.SaveGame`)))
  (`GameplayStatics.SaveGameToSlot` _asbp_save_game "SaveGame"))